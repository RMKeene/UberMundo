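; StaticMeshWrapper is an actor that wraps a static mesh component so it can be saved, restored and selected in a managed scene.
; ToMemento writes the mesh's asset path as a string compressed by the SceneManager found at BeginPlay.
; FromMemento decompresses it, loads and applies the mesh, or destroys the actor after a short delay if the cast fails.
; Selection functions toggle custom depth and stencil for highlighting.
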(event EventBeginPlay
  (Variables|Default|SetSceneManager (CallFunction|FindSceneManager)))

(event Collision|EventActorBeginOverlap
  (params (OtherActor :type Actor%20Object%20Reference)))

(event EventTick
  (params (DeltaSeconds :type Float%20%28single-precision%29)))

(event EventToMemento
  (params (ByteWriter :type Low%20Entry%20Byte%20Data%20Writer%20Object%20Reference) (Version :type Integer))
  (Class|LowEntryByteDataWriter|AddStringUtf8 ByteWriter (Default|CompressAssetName (Variables|Default|GetSceneManager) (Utilities|String|ToString(Name) (.objectpath (Class|AssetRegistryHelpers|CreateAssetData (Variables|/Script/Engine.StaticMeshComponent|GetStaticMesh (Variables|Default|GetStaticMesh)) false))))))

(event EventFromMemento
  (params (Byte%20Reader :type Low%20Entry%20Byte%20Data%20Reader%20Object%20Reference) (Version :type Integer))
  (bind _returnvalue (Class|LowEntryByteDataReader|GetStringUtf8 Byte%20Reader))
  (bind _uobject (Default|EnsureAssetLoaded (Variables|Default|GetSceneManager) (Default|DecompressAssetName (Variables|Default|GetSceneManager) _returnvalue)))
  (bind _asstatic_mesh (Utilities|Casting|CastToStaticMesh _uobject)
    (:then
      (Components|StaticMesh|SetStaticMesh (Variables|Default|GetStaticMesh) _asstatic_mesh))
    (:CastFailed
      (Utilities|FlowControl|Delay 0.2) ; No longer a valid static mesh.
      (Actor|DestroyActor))))

(fn ConstructionScript)

(fn EndSelection
  (bind _staticmesh (Variables|Default|GetStaticMesh))
  (Rendering|SetCustomDepthStencilValue _staticmesh 0)
  (Rendering|SetRenderCustomDepth _staticmesh false)
  (return true))

(fn StartSelection
  (bind _staticmesh (Variables|Default|GetStaticMesh))
  (Rendering|SetCustomDepthStencilValue _staticmesh 2)
  (Rendering|SetRenderCustomDepth _staticmesh true)
  (return true))